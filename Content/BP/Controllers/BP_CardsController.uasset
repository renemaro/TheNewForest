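; Player controller that builds and runs a grid-based card table with mouse input.
; On BeginPlay it expands the GameInstance's level deck counts into a shuffled list, puts a START row first, and spawns BP_Cards in hard-coded rows of six, marked unfinished.
; InitGame hides and locks all cards, then uses index offsets to make the chosen card's side and next-row neighbours movable, without edge checks.
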(event `self.ReceiveBeginPlay`
  (`WidgetBlueprintLibrary.SetInputMode_GameAndUIEx` self null "LockAlways")
  (set `self.bShowMouseCursor` true)
  (set `self.bEnableClickEvents` true)
  (`self.PlaceCardsOnMap` 6))

(event `/Game/Interfaces/INT_CardController.InitGame`
  (params (StartingCard :type "/Game/BP/BP_Card Object Reference"))
  (for _array_element (`self.CardsOnTable`)
    (message `/Game/Interfaces/INT_Card.SetVisibility` _array_element false)
    (message `/Game/Interfaces/INT_Card.CanMove` _array_element false))
  (`self.ActivateCardsArowndSelected` StartingCard 6))

(fn `ActivateCardsArowndSelected`
  (params (SelectedCard :type "/Game/BP/BP_Card Object Reference (by ref)") (Rows :type Integer))
  (locals (`CardPosition(local)` :type Integer) (`CardtSoActivate(local)` :type "Array of /Game/BP/BP_Card Object Reference"))
  (bind _output_get (set `local.CardPosition(local)` (`KismetArrayLibrary.Array_Find` (`self.CardsOnTable`) SelectedCard)))
  (`KismetArrayLibrary.Array_Add` (`local.CardtSoActivate(local)`) (`|GetArrayItem` (`self.CardsOnTable`) (+ _output_get (`local.Rows`))))
  (`|ExecutionSequence`
    (:`then_0`
      (`KismetArrayLibrary.Array_Add` (`local.CardtSoActivate(local)`) (`|GetArrayItem` (`self.CardsOnTable`) (+ (+ (`local.CardPosition(local)`) (`local.Rows`)) 1))))
    (:`then_1`
      (`KismetArrayLibrary.Array_Add` (`local.CardtSoActivate(local)`) (`|GetArrayItem` (`self.CardsOnTable`) (+ (+ (`local.CardPosition(local)`) (`local.Rows`)) -1))))
    (:`then_2`
      (`KismetArrayLibrary.Array_Add` (`local.CardtSoActivate(local)`) (`|GetArrayItem` (`self.CardsOnTable`) (+ (`local.CardPosition(local)`) 1))))
    (:`then_3`
      (`KismetArrayLibrary.Array_Add` (`local.CardtSoActivate(local)`) (`|GetArrayItem` (`self.CardsOnTable`) (+ (`local.CardPosition(local)`) -1))))
    (:`then_6`
      (for _array_element (`local.CardtSoActivate(local)`)
        (message `/Game/Interfaces/INT_Card.CanMove` _array_element true))
      (return))))

(fn `PlaceCardsOnMap`
  (params (Colums :type Integer))
  (locals (`DeckData(local)` :type "Map of Name to Integer") (`Colums(local)` :type Integer) (`Yoffset(local)` :type Integer :default -100))
  (bind _leveldeck (`self.LevelDeck`))
  (bind _returnvalue (+ (`local.Yoffset(local)`) 100))
  (set `local.Colums(local)` Colums)
  ;[1 1 1] This is a preparation before placing the cards on the level table. Gets global card data for the current level, converts it into the string, and shuffles.
  (bind _leveldeck_2 (message `/Game/Interfaces/INT_GameInstance.GetLevelDeck` (`GameplayStatics.GetGameInstance`)))
  (bind _output_get (set `local.DeckData(local)` _leveldeck_2))
  (bind _keys (`BlueprintMapLibrary.Map_Keys` _output_get))
  (for _array_element _keys
    (for _ (range 1 (+ (`BlueprintMapLibrary.Map_Find` (`local.DeckData(local)`) _array_element) 1))
      (`KismetArrayLibrary.Array_Add` (`self.LevelDeck`) _array_element)))
  (`KismetArrayLibrary.Array_Shuffle` (`self.LevelDeck`))
  ;[0.9635 1 0.9271] Adding the 'player start location' cards and reverse to move start row to the left
  (for _ (range 1 (+ (`local.Colums(local)`) 1))
    (`KismetArrayLibrary.Array_Add` _leveldeck "START"))
  (`KismetArrayLibrary.Array_Reverse` _leveldeck)
  ;[0.03215 0.8703 1] Spawning the cards. WARNING! This isn't a completed block because I need to figure out how to set the number of level cards structure and colums.
  (for (_array_element_2 _array_index) (`self.LevelDeck`)
    (set `local.Yoffset(local)` _returnvalue)
    (if (== _returnvalue 700)
      (set `local.Yoffset(local)` 0))
    (bind _returnvalue_2 (`|SpawnActorFromClass` "/Game/BP/BP_Card.BP_Card_C" (`KismetMathLibrary.MakeTransform` (`KismetMathLibrary.MakeVector` (`KismetMathLibrary.Conv_IntToDouble` (* (/ _array_index 6) 100)) (`KismetMathLibrary.Conv_IntToDouble` (`local.Yoffset(local)`)) 5.0)) "AlwaysSpawn" "MultiplyWithRoot" null _array_element_2 null))
    (`KismetArrayLibrary.Array_Add` (`self.CardsOnTable`) _returnvalue_2)))

(fn `UserConstructionScript`)